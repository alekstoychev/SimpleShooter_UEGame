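; BP_AmmoPickup is an ammo box pickup that resupplies player-controlled actors that overlap its sphere.
; On overlap while off cooldown, it calls AmmoPickup on the instigator's ShooterPlayerController.
; A successful pickup swaps the box to an inactive material and starts a timer that later calls ResetCooldown to restore the active material and re-enable pickup.
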(event `self.Sphere.OnComponentBeginOverlap`
  (params (OverlappedComponent :type "PrimitiveComponent Object Reference") (OtherActor :type "Actor Object Reference") (OtherComp :type "PrimitiveComponent Object Reference") (OtherBodyIndex :type Integer) (bFromSweep :type Boolean) (SweepResult :type "HitResult Structure (by ref)"))
  (if (not (`self.IsOnCooldown`))
    (bind _asshooter_player_controller (cast `ShooterPlayerController` (`self.GetInstigatorController` OtherActor)))
    (bind _bhaspackedup (`ShooterPlayerController.AmmoPickup` _asshooter_player_controller))
    (if _bhaspackedup
      (`PrimitiveComponent.SetMaterial` (`self.AmmoBox`) 0 "/Game/SimpleShooter/Assets/AmmoBox/M_AmmoBox_Inactive.M_AmmoBox_Inactive")
      (set `self.IsOnCooldown` true)
      (`KismetSystemLibrary.K2_SetTimer` null "ResetCooldown" 10.0))))

(fn `ResetCooldown`
  (set `self.IsOnCooldown` false)
  (`PrimitiveComponent.SetMaterial` (`self.AmmoBox`) 0 "/Game/SimpleShooter/Assets/AmmoBox/M_AmmoBox_Active.M_AmmoBox_Active"))

(fn `UserConstructionScript`)